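; Zombie-animated NPC that detects the third-person player character and provides a melee attack.
; Pawn Sensing sight and hearing store the enemy, then clear it through a 0.6-second retriggerable delay.
; Attack montage notifies toggle the attacking flag, with Attack_End starting and BeginAttack ending it.
; While attacking, Tick sphere-traces between right-hand sockets and only prints on a player hit, applying no damage.
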(event `self.PawnSensing.OnSeePawn`
  (params (Pawn :type "Pawn Object Reference"))
  (`self.GetEnemy` Pawn)
  (`KismetSystemLibrary.RetriggerableDelay` 0.6)
  (`self.ResetEnemy` null))

(event `self.PawnSensing.OnHearNoise`
  (params (Instigator :type "Pawn Object Reference") (Location :type "Vector Structure (by ref)") (Volume :type "Float (single-precision)"))
  (`self.GetEnemy` Instigator)
  (`KismetSystemLibrary.RetriggerableDelay` 0.6)
  (`self.ResetEnemy` null))

(event `Attack`
  (if (not (`self.IsAttacking`))
    (bind _notifyname (`|PlayMontage` (`self.Mesh`) "/Game/Fantasma/Animations/Zombie_Attack_Montage.Zombie_Attack_Montage" 1.0 0.0 "None" false)
      (:`OnNotifyBegin`
        (if (== _notifyname "Attack_End")
          (`self.startAttack`)
          (elif (== _notifyname "BeginAttack")
            (`self.EndAttack`)))))))

(event `startAttack`
  (set `self.IsAttacking` true)
  (`KismetSystemLibrary.PrintString` "InicioAttack"))

(event `EndAttack`
  (set `self.IsAttacking` false)
  (`KismetSystemLibrary.PrintString` "FinAttack"))

(event `self.ReceiveTick`
  (params (DeltaSeconds :type "Float (single-precision)"))
  (bind _mesh (`self.Mesh`))
  (if (`self.IsAttacking`)
    (bind _outhit (`KismetSystemLibrary.SphereTraceSingleForObjects` (`SceneComponent.GetSocketLocation` _mesh "InitDamageRightHandSocket") (`SceneComponent.GetSocketLocation` _mesh "EndDamageRightHandSocket") 5.0 (`|MakeArray` "ObjectTypeQuery3" :!type "EObjectTypeQuery Enum")))
    (cast `/Game/Bob/Blueprint/BP_ThirdPersonCharacter` (`.HitActor` (`GameplayStatics.BreakHitResult` _outhit)))
    (`KismetSystemLibrary.PrintString` "App Damage")))

(fn `GetEnemy`
  (params (enemy :type "Object Object Reference"))
  (bind _asbp_third_person_character (cast `/Game/Bob/Blueprint/BP_ThirdPersonCharacter` enemy))
  (set `self.SeeEnemy` _asbp_third_person_character)
  (set `self.ISeeEnemy` true))

(fn `ResetEnemy`
  (params (null :type "/Game/Bob/Blueprint/BP_ThirdPersonCharacter Object Reference"))
  (set `self.ISeeEnemy` false)
  (set `self.SeeEnemy` null))

(fn `UserConstructionScript`)
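; BP_NPC1 is an enemy NPC that detects the third-person player character and deals melee damage.
; PawnSensing sight and noise events store the player as the seen enemy, and a retriggerable delay clears it 0.6 seconds after the last stimulus.
; Attack plays a montage whose BeginAttack notify opens the damage window.
; During that window, Tick sphere-traces between right-hand sockets, applying damage and closing the window on hitting the player.
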(event `self.PawnSensing.OnSeePawn`
  (params (Pawn :type "Pawn Object Reference"))
  ; ViewEnemy
  (`self.GetEnemy` Pawn)
  (`KismetSystemLibrary.RetriggerableDelay` 0.6)
  (`self.ResetEnemy` null))

(event `self.PawnSensing.OnHearNoise`
  (params (Instigator :type "Pawn Object Reference") (Location :type "Vector Structure (by ref)") (Volume :type "Float (single-precision)"))
  ; ViewEnemy
  (`KismetSystemLibrary.PrintString` "Te escucho")
  (`self.GetEnemy` Instigator)
  (`KismetSystemLibrary.RetriggerableDelay` 0.6)
  (`self.ResetEnemy` null))

(event `Attack`
  ; AnimationMontageAttack
  (if (not (`self.IsAttacking`))
    (bind _notifyname (`|PlayMontage` (`self.Mesh`) "/Game/Interceptor/Animations/Attack_Interceptor_Montage.Attack_Interceptor_Montage" 1.0 1.0 "None" false)
      (:`OnNotifyBegin`
        (if (== _notifyname "BeginAttack")
          (`self.startAttack`))))))

(event `startAttack`
  ; Event IsAttack
  (set `self.IsAttacking` true)
  (`KismetSystemLibrary.PrintString` "InicioAttack"))

(event `EndAttack`
  ; Event IsAttack
  (set `self.IsAttacking` false)
  (`KismetSystemLibrary.PrintString` "FinAttack"))

(event `self.ReceiveTick`
  (params (DeltaSeconds :type "Float (single-precision)"))
  (bind _mesh (`self.Mesh`))
  ; AttackEvent
  (if (`self.IsAttacking`)
    (bind _outhit (`KismetSystemLibrary.SphereTraceSingleForObjects` :`Start` (`SceneComponent.GetSocketLocation` _mesh "InitDamageRightHandSocket") :`End` (`SceneComponent.GetSocketLocation` _mesh "EndDamageRightHandSocket") :`Radius` 5.0 :`ObjectTypes` (`|MakeArray` "ObjectTypeQuery3" :!type "EObjectTypeQuery Enum") :`DrawDebugType` "ForDuration"))
    (bind _asbp_third_person_character (cast `/Game/Bob/Blueprint/BP_ThirdPersonCharacter` (`.HitActor` (`GameplayStatics.BreakHitResult` _outhit))))
    (`GameplayStatics.ApplyDamage` _asbp_third_person_character (`self.damage`))
    (`self.EndAttack`)
    (`KismetSystemLibrary.PrintString` "Hello")))

(fn `GetEnemy`
  (params (enemy :type "Object Object Reference"))
  (bind _asbp_third_person_character (cast `/Game/Bob/Blueprint/BP_ThirdPersonCharacter` enemy))
  (set `self.SeeEnemy` _asbp_third_person_character)
  (set `self.ISeeEnemy` true))

(fn `ResetEnemy`
  (params (null :type "/Game/Bob/Blueprint/BP_ThirdPersonCharacter Object Reference"))
  (set `self.ISeeEnemy` false)
  (set `self.SeeEnemy` null))

(fn `UserConstructionScript`)
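; BP_NPC is a zombie-animated enemy that detects the player character by sight or hearing and can play an attack.
; PawnSensing events store a detected BP_ThirdPersonCharacter as SeeEnemy and set ISeeEnemy.
; Retriggerable delays clear that target shortly after sensing stops, acting as a brief memory.
; The Attack event plays a one-shot animation behind a short IsAttacking lockout, with no damage or movement logic here.
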(event `self.PawnSensing.OnSeePawn`
  (params (Pawn :type "Pawn Object Reference"))
  (`self.GetEnemy` Pawn)
  (`KismetSystemLibrary.RetriggerableDelay` 0.6)
  (`self.ResetEnemy` null))

(event `self.PawnSensing.OnHearNoise`
  (params (Instigator :type "Pawn Object Reference") (Location :type "Vector Structure (by ref)") (Volume :type "Float (single-precision)"))
  (`self.GetEnemy` Instigator)
  (`KismetSystemLibrary.RetriggerableDelay` 0.6)
  (`self.ResetEnemy` null))

(event `Attack`
  (if (not (`self.IsAttacking`))
    (set `self.IsAttacking` true)
    (`SkeletalMeshComponent.PlayAnimation` (`self.Mesh`) "/Game/Interceptor/Animations/Zombie_Attack.Zombie_Attack" false)
    (`KismetSystemLibrary.Delay` 0.2)
    (set `self.IsAttacking` false)))

(fn `GetEnemy`
  (params (enemy :type "Object Object Reference"))
  (bind _asbp_third_person_character (cast `/Game/ThirdPerson/Blueprints/BP_ThirdPersonCharacter` enemy))
  (set `self.SeeEnemy` _asbp_third_person_character)
  (set `self.ISeeEnemy` true))

(fn `ResetEnemy`
  (params (null :type "/Game/ThirdPerson/Blueprints/BP_ThirdPersonCharacter Object Reference"))
  (set `self.ISeeEnemy` false)
  (set `self.SeeEnemy` null))

(fn `UserConstructionScript`)